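; Pixel Streaming message handler for E3DS that receives input events from the streaming client.
; Each message is rebroadcast raw, decoded as JSON and routed by its Type field to on-screen keyboard commit or device info handling, with incompatible messages printed.
; Device info is cached for the session, so requests reuse it or query the client over Pixel Streaming.
; A mobile check reads the cached OS name, assuming desktop when info is missing.
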(event Custom|EventOnMessageReceived
  (params (Descriptor :type String))
  (Default|CallE3DSPXSonMessageReceived Descriptor)
  (Class|E3DSJsonObject|DecodeJson (Variables|Default|GetReceivedMessageJsonObject) Descriptor)
  (Utilities|DecodeJsonObject
    (:IncompatibleMessage
      (Development|PrintString Descriptor true true "(R=1.000000,G=0.090672,B=0.000000,A=1.000000)"))
    (:OnScreenKeyboardTextCommited
      (CallFunction|OnTextCommitedUsingonScreenKeyboard))
    (:takeUserDeviceInfo
      (CallFunction|OnTakeUserDeviceInfo))))

(event Custom|OnTextCommitedUsingOnScreenKeyboard
  (Default|CallE3DSPXSTextCommitedUsingonScreenKeyboard (Class|E3DSJsonObject|GetStringField (Variables|Default|GetReceivedMessageJsonObject) "value") (Class|E3DSJsonObject|GetStringField (Variables|Default|GetReceivedMessageJsonObject) "id")))

(event Custom|OnTakeUserDeviceInfo
  (bind _receivedmessagejsonobject (Variables|Default|GetReceivedMessageJsonObject))
  (bind _returnvalue (Class|E3DSJsonObject|GetObjectField _receivedmessagejsonobject "userDeviceInfo"))
  (bind _returnvalue_2 (Class|E3DSJsonObject|GetObjectField _returnvalue "os"))
  (Variables|Default|SetUserDeviceInfo (Variables|Default|GetReceivedMessageJsonObject))
  (Variables|Default|SetUserInfo_OS_Name (Class|E3DSJsonObject|GetStringField _returnvalue_2 "name"))
  (Variables|Default|SetUserInfo_OS_ShortName (Class|E3DSJsonObject|GetStringField _returnvalue_2 "short_name"))
  (Variables|Default|SetUserInfo_OS_Version (Class|E3DSJsonObject|GetStringField _returnvalue_2 "version"))
  (Variables|Default|SetUserInfo_Client_BrowserName (Class|E3DSJsonObject|GetStringField (Class|E3DSJsonObject|GetObjectField _returnvalue "client") "name")))

(event EventBeginPlay
  (EventDispatchers|BindEventtoOnInputEvent (Variables|Default|GetPixelStreamingInput) (delegate Custom|EventOnMessageReceived))
  (bind _returnvalue (Game|ConstructObjectfromClass "/Script/E3DSFeatures.E3DSJsonObject"))
  (Variables|Default|SetReceivedMessageJsonObject _returnvalue))

(fn ConstructionScript)

(fn E3DSRequestDeviceInfo
  (Utilities|IsValid (Variables|Default|GetUserDeviceInfo)
    (:Is%20Valid
      ;[1 1 1] User Device Wont change in the middle of a session so just use the old data again
      (Variables|Default|SetReceivedMessageJsonObject (Variables|Default|GetUserDeviceInfo))
      (CallFunction|OnTakeUserDeviceInfo))
    (:Is%20Not%20Valid
      (Class|PixelStreamingInput|SendPixelStreamingResponse (Variables|Default|GetPixelStreamingInput) (Utilities|String|MakeLiteralString "{\"cmd\":\"sendDeviceInfo\",\"value\":\"\"}")))))

(fn E3DSIsClientMobileDevice?
  (Utilities|IsValid (Variables|Default|GetUserDeviceInfo)
    (:Is%20Valid
      (switch string (Variables|Default|GetUserInfo_OS_Name)
        (:Default
          _)
        (:Android
          (return true))
        (:iOS
          (return true))))
    (:Is%20Not%20Valid
      (Development|PrintString "E3DS ERROR : User device info is not received yet. considering desktop request user device info or wait for previous request to get a response" true true "(R=1.000000,G=0.000000,B=0.005000,A=1.000000)" 5.0)))
  (return false))